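; Flame pillar actor whose point light flickers with varying intensity.
; On BeginPlay it randomly picks one of two timelines and plays it from the start, choosing again whenever one finishes for an endless, non-uniform loop.
; Each timeline update feeds its float track to SetLightIntensity, which scales the point light's intensity relative to BaseIntensity.
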(event `self.ReceiveBeginPlay`
  (`self.ChooseTimeline`))

(event `ChooseTimeline`
  (switch `int` (`KismetMathLibrary.RandomIntegerInRange` 0 1)
    (:`0`
      (`self.StartTimeLine1`))
    (:`1`
      (`self.StartTimeLine2`))))

(event `StartTimeLine1`
  (bind (_direction _newtrack_0) (`Timeline|FlameIntensityTimeline` :!via `PlayFromStart`)
    (:`Update`
      (`self.SetLightIntensity` _newtrack_0))
    (:`Finished`
      (`self.ChooseTimeline`))))

(event `StartTimeLine2`
  (bind (_direction _newtrack_0) (`Timeline|Timeline` :!via `PlayFromStart`)
    (:`Update`
      (`self.SetLightIntensity` _newtrack_0))
    (:`Finished`
      (`self.ChooseTimeline`))))

(fn `SetLightIntensity`
  (params (A :type "Float (double-precision)"))
  (`LightComponent.SetIntensity` (`self.PointLight`) (* A (`self.BaseIntensity`))))

(fn `UserConstructionScript`)